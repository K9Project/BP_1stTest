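; Actor with two cube components that rotates one or the other every frame, selected by the RotateFirstCube boolean.
; Tick branches on the flag and calls a separate function per cube, each adding a fixed world rotation on a different axis.
; The first cube's rotation passes through a DoN that is never reset, so it stops after 120 calls, while the second has no limit.
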(event EventBeginPlay)

(event Collision|EventActorBeginOverlap
  (params (OtherActor :type Actor%20Object%20Reference)))

(event EventTick
  (params (DeltaSeconds :type Float%20%28single-precision%29))
  (if (Variables|Default|GetRotateFirstCube)
    (Utilities|FlowControl|DoN 120
      (:Exit
        (CallFunction|RotateFirstCubeFunc)))
    (else
      (CallFunction|RotateSecondCubeFunc))))

(fn ConstructionScript)

(fn RotateFirstCubeFunc
  (Transformation|AddWorldRotation (Variables|Default|GetCube) "10.000000, 0, 0" false false))

(fn RotateSecondCubeFunc
  (Transformation|AddWorldRotation (Variables|Default|GetCube1) "0.000000,10.000000, 0" false false))